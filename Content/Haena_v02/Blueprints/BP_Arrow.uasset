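; BP_Arrow is an arrow projectile that can be held still and then launched.
; On BeginPlay, StopProjectile zeroes its local velocity and gravity on the ProjectileMovement component and deactivates its particle system.
; StartProjectile fires it along local X with high speed and partial gravity, activates the particles, and swaps the arrow mesh to an emissive material.
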(event `self.ReceiveBeginPlay`
  (`self.Stop Projectile`))

(event `Stop Projectile`
  (bind _projectilemovement (`self.ProjectileMovement`))
  (bind _output_get (set `self.Arrow Velocity` (0.0 0.0 0.0)))
  (`ProjectileMovementComponent.SetVelocityInLocalSpace` _projectilemovement _output_get)
  (set `ProjectileMovementComponent.ProjectileGravityScale` 0.0 _projectilemovement)
  (`ActorComponent.Deactivate` (`self.ParticleSystem`)))

(event `Start Projectile`
  (bind _projectilemovement (`self.ProjectileMovement`))
  (bind _output_get (set `self.Arrow Velocity` (7000.0 0.0 0.0)))
  (`ProjectileMovementComponent.SetVelocityInLocalSpace` _projectilemovement _output_get)
  (set `ProjectileMovementComponent.ProjectileGravityScale` 0.5 _projectilemovement)
  (`ActorComponent.Activate` (`self.ParticleSystem`) false)
  (`PrimitiveComponent.SetMaterial` (`self.SK_Arrow`) 0 "/Game/Haena_v02/Materials/Weapons_ETC/MI_Arrow_Emissive.MI_Arrow_Emissive"))

(fn `UserConstructionScript`)