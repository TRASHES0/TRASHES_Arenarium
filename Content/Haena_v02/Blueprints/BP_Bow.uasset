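; BP_Bow is a bow Blueprint that animates its skeletal mesh through the idle, string pull, aim and shoot states.
; Four events (Idle, PullString, Aim, Shoot) each play a different starting section of one shared montage on SKBow, with all but Idle at double speed.
; It holds only animation triggers, with no projectile or input logic and an empty construction script.
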(event `Aim`
  (`|PlayMontage` (`self.SK_Bow`) "/Game/Haena_v02/Animation/Bow/A_Bow_Anim_Montage.A_Bow_Anim_Montage" 2.0 0.0 "Pull_02"))

(event `Idle`
  (`|PlayMontage` (`self.SK_Bow`) "/Game/Haena_v02/Animation/Bow/A_Bow_Anim_Montage.A_Bow_Anim_Montage" 1.0 0.0 "Idle"))

(event `Shoot`
  (`|PlayMontage` (`self.SK_Bow`) "/Game/Haena_v02/Animation/Bow/A_Bow_Anim_Montage.A_Bow_Anim_Montage" 2.0 0.0 "Aim_End"))

(event `Pull String`
  (`|PlayMontage` (`self.SK_Bow`) "/Game/Haena_v02/Animation/Bow/A_Bow_Anim_Montage.A_Bow_Anim_Montage" 2.0 0.0 "Reload_Start"))

(fn `UserConstructionScript`)