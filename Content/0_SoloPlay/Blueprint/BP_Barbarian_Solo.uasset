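; BP_Barbarian_Solo is the solo-play Barbarian character, built on the MACS Gameplay Ability System setup.
; Tick mirrors the SwordAndShield combo gameplay tag into the Attacking flag.
; G and H act as AI perception triggers, making noise at the character or reporting a damage event on the first BP_Enemy_Base found.
; A SwordAndShield weapon-class effect application is present but unconnected.
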(event `self.ReceiveBeginPlay`)

(event `Key|G`
  (params (Key :type "Key Structure"))
  (:`Pressed`
    (`self.MakeNoise` 1.0 self (`self.K2_GetActorLocation`))))

(event `Key|H`
  (params (Key :type "Key Structure"))
  (:`Pressed`
    (bind _returnvalue (`GameplayStatics.GetActorOfClass` "/Game/0_SoloPlay/Blueprint/BP_Enemy_Base.BP_Enemy_Base_C"))
    (`AISense_Damage.ReportDamageEvent` _returnvalue self 10.0 (`self.K2_GetActorLocation`))))

(event `/Game/MACS/Classes/Interfaces/BPI_MACS_Character.SendGameplayEvent`
  (params (GameplayTag :type "GameplayTag Structure") (Payload :type "GameplayEventData Structure")))

(event `self.ReceiveTick`
  (params (DeltaSeconds :type "Float (single-precision)"))
  (if (`/Game/MACS/Classes/BPL_MACS.GameplayTagCheck` self (struct :`TagName` "MACS_GAS.Abilities.States.WeaponClass.SwordAndShield.Combo"))
    (set `self.Attacking` true)
    (else
      (set `self.Attacking` false))))

(fn `UserConstructionScript`
  (`parent.UserConstructionScript`))