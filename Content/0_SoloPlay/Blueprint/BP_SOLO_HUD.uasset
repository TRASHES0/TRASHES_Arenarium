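; Solo-play HUD that creates and manages the fade-in, game menu, combat UI, death and win widgets.
; BeginPlay binds a melee enemy and the player character to the solo UI, retrying every 0.2s until the player cast succeeds.
; ToggleWidget shows one listed menu at a time and switches input mode and cursor.
; Death shows a UI-only screen; winning clears the widgets, blocks toggling and shows Win_Solo after a delay.
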(event `self.ReceiveBeginPlay`
  (bind _returnvalue (`self.GetOwningPlayerController`))
  (`|ExecutionSequence`
    (:`then_0`
      (`WidgetBlueprintLibrary.SetInputMode_GameOnly` _returnvalue)
      (set `PlayerController.bShowMouseCursor` false _returnvalue)
      (bind _returnvalue_2 (`|CreateWidget` "/Game/BeginnerMultiplayerLobby/Widgets/General/WB_FadeInOut.WB_FadeInOut_C" _returnvalue))
      (`UserWidget.AddToViewport` _returnvalue_2 0)
      (`/Game/BeginnerMultiplayerLobby/Widgets/General/WB_FadeInOut.Fade In` _returnvalue_2))
    (:`then_1`
      (bind _returnvalue_3 (`|CreateWidget` "/Game/BeginnerMultiplayerLobby/Widgets/Gameplay/GameMenu/WB_GameMenu.WB_GameMenu_C" (`self.GetOwningPlayerController`)))
      (bind _output_get (set `self.Menu` _returnvalue_3))
      (`UserWidget.AddToViewport` _output_get 1)
      (`KismetArrayLibrary.Array_Add` (`self.GameMenu_WidgetList`) (`self.Menu`)))
    (:`then_2`
      (bind _returnvalue_4 (`|CreateWidget` "/Game/0_SoloPlay/Blueprint/WB_MACS_UI_SOLO.WB_MACS_UI_SOLO_C" (`self.GetOwningPlayerController`)))
      (`/Engine/EditorBlueprintResources/StandardMacros.IsValid` _returnvalue_4
        (:`Is Valid`
          (bind _output_get_2 (set `self.Solo UI` _returnvalue_4))
          (`UserWidget.AddToViewport` _output_get_2 0)
          (`|ExecutionSequence`
            (:`then_0`
              (bind _returnvalue_5 (`GameplayStatics.GetActorOfClass` "/Game/0_SoloPlay/Blueprint/BP_Enemy_Melee.BP_Enemy_Melee_C"))
              (`/Engine/EditorBlueprintResources/StandardMacros.IsValid` _returnvalue_5
                (:`Is Valid`
                  (set `/Game/MACS/UI/WB_MACS_CharData.PawnRef` _returnvalue_5 (`/Game/0_SoloPlay/Blueprint/WB_MACS_UI_SOLO.WB_ENEMY_DATA` _output_get_2)))))
            (:`then_1`
              (bind _asbp_macs_character_base (cast `/Game/MACS/Classes/BP_MACS_Character_Base` (`GameplayStatics.GetPlayerCharacter` 0) :!label _label)
                (:`then`
                  (`/Engine/EditorBlueprintResources/StandardMacros.IsValid` _asbp_macs_character_base
                    (:`Is Valid`
                      (set `/Game/MACS/UI/WB_MACS_CharData.PawnRef` _asbp_macs_character_base (`/Game/0_SoloPlay/Blueprint/WB_MACS_UI_SOLO.WB_CharData` _output_get_2)))))
                (:`CastFailed`
                  (`KismetSystemLibrary.Delay` 0.2)
                  (goto _label))))))))
    (:`then_3`
      (bind _returnvalue_6 (`|CreateWidget` "/Game/0_SoloPlay/Blueprint/Die_Solo.Die_Solo_C" (`self.GetOwningPlayerController`)))
      (set `self.Die` _returnvalue_6))
    (:`then_4`
      (bind _returnvalue_7 (`|CreateWidget` "/Game/BeginnerMultiplayerLobby/Widgets/Gameplay/UI/Win.Win_C" (`self.GetOwningPlayerController`)))
      (set `self.Win` _returnvalue_7))))

(event `Toggle_GameMenu`
  (if (not (`self.IsEnd`))
    (`self.ToggleWidget` (`self.Menu`))))

(event `/Game/BeginnerMultiplayerLobby/Blueprints/Interfaces/BP_INT_UserInterface.Forward_ToggleWidget`
  (params (TargetWidget :type "UserWidget Object Reference"))
  (if (not (`self.IsEnd`))
    (`self.ToggleWidget` TargetWidget)))

(event `ShowWidget`
  (bind _returnvalue (`GameplayStatics.GetPlayerController` 0))
  (`UserWidget.AddToViewport` (`self.Die`) 0)
  (`WidgetBlueprintLibrary.SetInputMode_UIOnlyEx` _returnvalue null "LockAlways")
  (set `PlayerController.bShowMouseCursor` true _returnvalue))

(event `CreateWin_Solo`
  (bind _returnvalue (`GameplayStatics.GetPlayerController` 0))
  (bind _returnvalue_2 (`GameplayStatics.GetPlayerController` 0))
  (bind _spectate (`self.Spectate`))
  (bind _solo_ui (`self.Solo UI`))
  (bind _die (`self.Die`))
  (bind _menu (`self.Menu`))
  (message `EnhancedInputSubsystemInterface.ClearAllMappings` _returnvalue)
  (`WidgetBlueprintLibrary.SetInputMode_UIOnlyEx` _returnvalue null "LockAlways")
  (`|ExecutionSequence`
    (:`then_0`
      (if (`KismetSystemLibrary.IsValid` _die)
        (`Widget.RemoveFromParent` _die)))
    (:`then_1`
      (if (`KismetSystemLibrary.IsValid` _spectate)
        (`Widget.RemoveFromParent` _spectate)))
    (:`then_2`
      (if (`KismetSystemLibrary.IsValid` _menu)
        (`Widget.RemoveFromParent` _menu)))
    (:`then_3`
      (if (`KismetSystemLibrary.IsValid` _solo_ui)
        (`Widget.RemoveFromParent` _solo_ui)))
    (:`then_4`
      (set `self.IsEnd` true)
      (`KismetSystemLibrary.Delay` 1.0)
      (bind _returnvalue_3 (`|CreateWidget` "/Game/BeginnerMultiplayerLobby/Widgets/Gameplay/UI/Win_Solo.Win_Solo_C" _returnvalue_2))
      (`UserWidget.AddToViewport` _returnvalue_3 0)
      (set `PlayerController.bShowMouseCursor` true _returnvalue_2))))

(fn `FocusGame`
  (bind _returnvalue (`self.GetOwningPlayerController`))
  ;[0.05098 0.05098 0.05098] Collapsed the current widget and sets input mode on the Game
  (`Widget.SetVisibility` (`self.CurrentWidget`) "Collapsed")
  (`WidgetBlueprintLibrary.SetInputMode_GameOnly` _returnvalue)
  (set `PlayerController.bShowMouseCursor` false _returnvalue))

(fn `FocusWidget`
  (bind _returnvalue (`self.GetOwningPlayerController`))
  ;[0.05098 0.05098 0.05098] Makes the current widget visible and sets input mode to the Game and new Widget
  (`Widget.SetVisibility` (`self.CurrentWidget`) "SelfHitTestInvisible")
  (`WidgetBlueprintLibrary.SetInputMode_GameAndUIEx` _returnvalue (`self.CurrentWidget`))
  (set `PlayerController.bShowMouseCursor` true _returnvalue))

(fn `ToggleWidget`
  (params (CurrentWidget :type "UserWidget Object Reference"))
  ;[0.05098 0.05098 0.05098] Sets the Current Widget and check if we have to Untoggle currently shown widgets, then we check if we focus the new widget or focus the game
  (set `self.CurrentWidget` CurrentWidget)
  (for _array_element (`self.GameMenu_WidgetList`)
    (`/Engine/EditorBlueprintResources/StandardMacros.IsValid` _array_element
      (:`Is Valid`
        (if (== (`local.CurrentWidget`) _array_element)
          (if (`Widget.IsVisible` (`local.CurrentWidget`))
            (`self.FocusGame`)
            (else
              (`self.FocusWidget`)))
          (elif (`Widget.IsVisible` _array_element)
            (`Widget.SetVisibility` _array_element "Collapsed")))))))

(fn `UserConstructionScript`)

(fn `커스텀이벤트`)