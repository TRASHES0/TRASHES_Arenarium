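; Base enemy character Blueprint that supplies movement and AI tuning data for solo-play enemies.
; Getter functions expose attack and defend radii and an assigned patrol route.
; Set Movement Speed maps idle, walking, jogging and sprinting states to the character's max walk speed.
; BeginPlay only calls the parent, and a leftover MaxHealth attribute assignment is never executed.
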(event `self.ReceiveBeginPlay`
  (`parent.ReceiveBeginPlay`))

(fn `Get Ideal Range`
  (returns (AttackRadius :type "Float (double-precision)") (DefendRadius :type "Float (double-precision)"))
  (return (`self.Attack Radius`) (`self.Defend Radius`)))

(fn `Get PatrolRoute`
  (returns (PatrolRoute :type "/Game/0_SoloPlay/Blueprint/BP_PatrolRoute Object Reference"))
  (return (`self.PatrolRoute`)))

(fn `Set Movement Speed`
  (params (Speed :type "/Game/0_SoloPlay/AI/Enum/E_MovementSpeed Enum" :default "NewEnumerator0"))
  (returns (SpeedValue :type "Float (double-precision)"))
  (set `CharacterMovementComponent.MaxWalkSpeed` (select `/Game/0_SoloPlay/AI/Enum/E_MovementSpeed` Speed :`NewEnumerator1` 200.0 :`NewEnumerator2` 400.0 :`NewEnumerator3` 600.0 :!type "Float (single-precision)") (`self.CharacterMovement`))
  (return 0.0))

(fn `UserConstructionScript`)