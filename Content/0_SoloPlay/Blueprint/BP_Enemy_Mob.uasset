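; Mob enemy character Blueprint that layers fighter setup, movement speeds and combat ranges onto its parent class.
; On BeginPlay it applies the Fighter weapon-class gameplay effect to itself through the MACS ability system component.
; Overrides map movement states to max walk speed and report a short attack radius with zero defend radius.
; Hit reactions are forwarded to a server-side setter and exposed through a getter.
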(event `self.ReceiveBeginPlay`
  (`parent.ReceiveBeginPlay`)
  (`AbilitySystemComponent.BP_ApplyGameplayEffectToSelf` :`self` (`self.MACS_AbilitySystemComponent`) :`GameplayEffectClass` "/Game/MACS/GAS/Effects/States/WeaponClass/GE_MACS_WeaponClass_Fighter.GE_MACS_WeaponClass_Fighter_C"))

(event `/Game/MACS/Classes/Interfaces/BPI_MACS_Character.SetHitReaction`
  (params (MACS_HitReaction :type "/Game/MACS/DataModels/S_MACS_HitReaction Structure"))
  (`self.SetHitReactionOnServer` MACS_HitReaction))

(fn `Get Ideal Range`
  (returns (AttackRadius :type "Float (double-precision)") (DefendRadius :type "Float (double-precision)"))
  (return 100.0 0.0))

(fn `GetHitReaction`
  (returns (GetHitReaction :type "/Game/MACS/DataModels/S_MACS_HitReaction Structure"))
  (return (`self.HitReaction`)))

(fn `Set Movement Speed`
  (params (Speed :type "/Game/0_SoloPlay/AI/Enum/E_MovementSpeed Enum" :default "NewEnumerator0"))
  (returns (SpeedValue :type "Float (double-precision)"))
  (set `CharacterMovementComponent.MaxWalkSpeed` (select `/Game/0_SoloPlay/AI/Enum/E_MovementSpeed` Speed :`NewEnumerator1` 200.0 :`NewEnumerator2` 400.0 :`NewEnumerator3` 600.0 :!type "Float (single-precision)") (`self.CharacterMovement`))
  (return 0.0))

(fn `UserConstructionScript`
  (`parent.UserConstructionScript`))