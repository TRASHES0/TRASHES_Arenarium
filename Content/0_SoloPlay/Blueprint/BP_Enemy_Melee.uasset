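; Melee enemy Blueprint named "디스트로이어" (Destroyer) that fights with a hammer, built on a parent enemy class.
; BeginPlay applies the hammer weapon-class Gameplay Effect through the MACS ability system component.
; Attack and equip events play montages and fire completion callbacks whether finished or interrupted, while unequip updates immediately.
; Attacks use a montage directly, as the hammer combo ability activation is disconnected debug logic.
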(event `self.ReceiveBeginPlay`
  (`parent.ReceiveBeginPlay`)
  (set `self.PlayerName` "디스트로이어")
  (`AbilitySystemComponent.BP_ApplyGameplayEffectToSelf` :`self` (`self.MACS_AbilitySystemComponent`) :`GameplayEffectClass` "/Game/0_SoloPlay/GameEffect/GE_MACS_WeaponClass_Hammer.GE_MACS_WeaponClass_Hammer_C"))

(event `/Game/0_SoloPlay/AI/BPI_EnemyAI.Attack`
  (`|PlayMontage` (`self.Mesh`) "/Game/0_SoloPlay/Animation/Hammer_Attack_2Combo_1_Montage.Hammer_Attack_2Combo_1_Montage"
    (:`OnCompleted`
      _)
    (:`OnInterrupted`
      _))
  (`self.OnAttackEnd`))

(event `self.ReceiveTick`
  (params (DeltaSeconds :type "Float (single-precision)")))

(event `/Game/0_SoloPlay/AI/BPI_EnemyAI.Equip Weapon`
  (`|PlayMontage` (`self.Mesh`) "/Game/Animation/SwordAnimsetPro/Animations/In-Place/Buff_out_Anim_Montage.Buff_out_Anim_Montage"
    (:`OnCompleted`
      _)
    (:`OnInterrupted`
      _))
  (`self.OnWeaponEquipped`)
  (set `self.IsWeaponEquiped` true))

(event `/Game/0_SoloPlay/AI/BPI_EnemyAI.Unequip Weapon`
  (`self.OnWeaponUnequipped`)
  (set `self.IsWeaponEquiped` false))

(fn `UserConstructionScript`
  (`parent.UserConstructionScript`))