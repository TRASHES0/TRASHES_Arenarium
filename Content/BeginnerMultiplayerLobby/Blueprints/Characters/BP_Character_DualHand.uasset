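; BP_Character_DualHand is a character Blueprint that adds a left-click ground melee combo and reports itself as not targetable.
; A click clears CanMelee and, unless the character is falling, plays the next montage from an array, wrapping the attack index after the last.
; CS_SaveMelee re-enables input to continue the combo, while CS_ResetMelee also restarts it; neither is called within this Blueprint.
; An airborne click still clears CanMelee without playing an attack.
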(event `Key|LeftMouseButton`
  (params (Key :type "Key Structure"))
  ;[1 0 0.03922] 마우스 왼쪽 클릭
  (:`Pressed`
    (if (`self.Can Melee`)
      (set `self.Can Melee` false)
      (if (not (`NavMovementComponent.IsFalling` (`self.CharacterMovement`)))
        (`self.CS_GroundComboMontage`)))))

(event `CS_SaveMelee`
  ;[1 0 0.03922] 마우스 왼쪽 클릭
  (set `self.Can Melee` true))

(event `CS_ResetMelee`
  ;[1 0 0.03922] 마우스 왼쪽 클릭
  (set `self.Can Melee` true)
  (set `self.Attack Count` 0))

(event `CS_GroundComboMontage`
  ;[1 0 0.03922] 마우스 왼쪽 클릭
  ;;[1 1 1] 콤보 몽타주
  (`self.PlayAnimMontage` self (`|GetArrayItem` (`self.Ground Combo Montage`) (`self.Attack Count`)) 1.0 "None")
  (if (>= (`self.Attack Count`) (- (`KismetArrayLibrary.Array_Length` (`self.Ground Combo Montage`)) 1))
    (set `self.Attack Count` 0)
    (else
      (`/Engine/EditorBlueprintResources/StandardMacros.IncrementInt` (`self.Attack Count`)))))

(fn `IsTargetable`
  (returns (ReturnValue :type Boolean))
  (return false))

(fn `UserConstructionScript`
  (`parent.UserConstructionScript`))