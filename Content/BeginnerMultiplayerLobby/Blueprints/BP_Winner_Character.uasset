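; BP_Winner_Character is a character Blueprint, apparently for showing a match winner, that assigns an animation Blueprint to suit the character type.
; ChangeAnim tests the display name of its Mesh for known character-name substrings in an if/else chain and sets the corresponding anim class.
; An unmatched name prints a failure message.
; ChangeTransform, BeginPlay, Tick, overlap and the construction script are empty.
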(event `ChangeTransform`)

(event `ChangeAnim`
  (bind _mesh (`self.Mesh`))
  (bind _returnvalue (`KismetSystemLibrary.GetDisplayName` _mesh))
  (if (`KismetStringLibrary.Contains` _returnvalue "SAMURAIGIRL")
    (`SkeletalMeshComponent.SetAnimInstanceClass` _mesh "/Game/Characters_Animation_Retarget/Samurai/2_ABP_MACS.2_ABP_MACS_C")
    (elif (`KismetStringLibrary.Contains` _returnvalue "Ordinary")
      (`SkeletalMeshComponent.SetAnimInstanceClass` _mesh "/Game/Characters_Animation_Retarget/GreatAxe/Axe_ABP_MACS.Axe_ABP_MACS_C")
      (elif (`KismetStringLibrary.Contains` _returnvalue "Mafia")
        (`SkeletalMeshComponent.SetAnimInstanceClass` _mesh "/Game/Characters_Animation_Retarget/Fighter/0_ABP_MACS.0_ABP_MACS_C")
        (elif (`KismetStringLibrary.Contains` _returnvalue "Barbarian")
          (`SkeletalMeshComponent.SetAnimInstanceClass` _mesh "/Game/Characters_Animation_Retarget/Sword/1_ABP_MACS.1_ABP_MACS_C")
          (elif (`KismetStringLibrary.Contains` _returnvalue "Wukong")
            (`SkeletalMeshComponent.SetAnimInstanceClass` _mesh "/Game/Characters_Animation_Retarget/Wukong/0Wukong_ABP_MACS.0Wukong_ABP_MACS_C")
            (elif (`KismetStringLibrary.Contains` _returnvalue "Haena")
              (`SkeletalMeshComponent.SetAnimInstanceClass` _mesh "/Game/Characters_Animation_Retarget/Haena/Haena_ABP_MACS.Haena_ABP_MACS_C")
              (else
                (`KismetSystemLibrary.PrintString` "animation load fail")))))))))

(event `self.ReceiveBeginPlay`)

(fn `UserConstructionScript`)