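; Base player state for a multiplayer lobby game, holding each player's replicated ready flag, death flag, character and player number.
; Changes to the ready and death flags fire RepNotifies that, only on the authority, have BP_GS_Base run CheckReady or CheckDead.
; The player number notify just prints a debug string, and the character notify and event graph are empty.
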(fn `OnRep_IsDead`
  (`/Engine/EditorBlueprintResources/ActorMacros.Switch Has Authority`
    (:`Authority`
      (bind _asbp_gs_base (cast `/Game/BeginnerMultiplayerLobby/Blueprints/GameModes/Base/Core/BP_GS_Base` (`GameplayStatics.GetGameState`)))
      (`/Game/BeginnerMultiplayerLobby/Blueprints/GameModes/Base/Core/BP_GS_Base.Check Dead` _asbp_gs_base))))

(fn `OnRep_IsReady`
  (`/Engine/EditorBlueprintResources/ActorMacros.Switch Has Authority`
    (:`Authority`
      (bind _asbp_gs_base (cast `/Game/BeginnerMultiplayerLobby/Blueprints/GameModes/Base/Core/BP_GS_Base` (`GameplayStatics.GetGameState`)))
      (`/Game/BeginnerMultiplayerLobby/Blueprints/GameModes/Base/Core/BP_GS_Base.Check_Ready` _asbp_gs_base))))

(fn `OnRep_PlayerCharacter`)

(fn `OnRep_PlayerNum`
  (`KismetSystemLibrary.PrintString` (`KismetStringLibrary.Concat_StrStr` "Player NUM:" (`KismetStringLibrary.Conv_IntToString` (`self.PlayerNum`)))))

(fn `UserConstructionScript`)