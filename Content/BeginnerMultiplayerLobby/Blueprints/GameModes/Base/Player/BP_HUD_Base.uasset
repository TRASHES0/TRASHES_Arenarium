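; Base HUD for the multiplayer lobby template that creates the in-game menu widget and manages toggling it.
; BeginPlay sets game-only input, adds WB_GameMenu to the viewport and registers it in a widget list.
; ToggleWidget collapses other listed widgets, then shows or hides the target.
; Showing switches to game-and-UI input with the mouse cursor, while hiding returns game-only input and hides the cursor.
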(event `self.ReceiveBeginPlay`
  ;[0.05098 0.05098 0.05098] Focus input on game
  (`WidgetBlueprintLibrary.SetInputMode_GameOnly` (`self.GetOwningPlayerController`))
  ;[0.05448 0.05448 0.05448] Add this widget to the Viewport and to the GameMenu_WidgetList
  (bind _returnvalue (`|CreateWidget` "/Game/BeginnerMultiplayerLobby/Widgets/Gameplay/GameMenu/WB_GameMenu.WB_GameMenu_C" (`self.GetOwningPlayerController`)))
  (bind _output_get (set `self.WB_GameMenu` _returnvalue))
  (`UserWidget.AddToViewport` _output_get 1)
  (`KismetArrayLibrary.Array_Add` (`self.GameMenu_WidgetList`) (`self.WB_GameMenu`)))

(event `/Game/BeginnerMultiplayerLobby/Blueprints/Interfaces/BP_INT_UserInterface.Forward_ToggleWidget`
  (params (TargetWidget :type "UserWidget Object Reference"))
  ;[0.05448 0.05448 0.05448] Toggle Widget events
  (`self.ToggleWidget` TargetWidget))

(event `Toggle_GameMenu`
  ;[0.05448 0.05448 0.05448] Toggle Widget events
  (`self.ToggleWidget` (`self.WB_GameMenu`)))

(fn `FocusGame`
  (bind _returnvalue (`self.GetOwningPlayerController`))
  ;[0.05098 0.05098 0.05098] Collapsed the current widget and sets input mode on the Game
  (`Widget.SetVisibility` (`self.CurrentWidget`) "Collapsed")
  (`WidgetBlueprintLibrary.SetInputMode_GameOnly` _returnvalue)
  (set `PlayerController.bShowMouseCursor` false _returnvalue))

(fn `FocusWidget`
  (bind _returnvalue (`self.GetOwningPlayerController`))
  ;[0.05098 0.05098 0.05098] Makes the current widget visible and sets input mode to the Game and new Widget
  (`Widget.SetVisibility` (`self.CurrentWidget`) "SelfHitTestInvisible")
  (`WidgetBlueprintLibrary.SetInputMode_GameAndUIEx` _returnvalue (`self.CurrentWidget`))
  (set `PlayerController.bShowMouseCursor` true _returnvalue))

(fn `ToggleWidget`
  (params (CurrentWidget :type "UserWidget Object Reference"))
  ;[0.05098 0.05098 0.05098] Sets the Current Widget and check if we have to Untoggle currently shown widgets, then we check if we focus the new widget or focus the game
  (set `self.CurrentWidget` CurrentWidget)
  (for _array_element (`self.GameMenu_WidgetList`)
    (`/Engine/EditorBlueprintResources/StandardMacros.IsValid` _array_element
      (:`Is Valid`
        (if (== (`self.CurrentWidget`) _array_element)
          (if (`Widget.IsVisible` (`self.CurrentWidget`))
            (`self.FocusGame`)
            (else
              (`self.FocusWidget`)))
          (elif (`Widget.IsVisible` _array_element)
            (`Widget.SetVisibility` _array_element "Collapsed")))))))

(fn `UserConstructionScript`)