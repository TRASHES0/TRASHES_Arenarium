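; Base lobby Game State that tracks the player list and runs the ready-check countdown to match start.
; BP_GM_Base login/logout events update the replicated player list, whose RepNotify refreshes every WB_PlayerList widget.
; CheckReady compares ready PlayerStates against the session's connection count to set StartCheck.
; Authority-only RepNotifies drive a self-repeating one-second countdown, calling SRSpawnCharacter on player controller 0 at zero.
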(event `Update_PlayerList`
  ;[0.05448 0.05448 0.05448] Called By 'BP_GM_Base' OnLogin/Logout events
  (set `self.AllPlayer` (`self.PlayerArray`)))

(event `CountDownStart`
  (`KismetSystemLibrary.Delay` 1.0)
  (set `self.CountDown` (- (`self.CountDown`) 1)))

(fn `check_ready`
  ;[0.05098 0.05098 0.05098] Reset the Ready Status variables since we're checking again
  (set `self.ReadyCount` 0)
  (set `self.CountDown` 5)
  (set `self.StartCheck` false)
  ;[0.05098 0.05098 0.05098] Count the amount of players who's Ready Status is set to Ready. Then determine if we Start the Game Launch or not.
  (for _array_element (`self.PlayerArray`)
    (bind _numconnections (`AdvancedSessionsLibrary.GetSessionSettings`)
      (:`OnSuccess`
        (bind _asbp_ps_base (cast `/Game/BeginnerMultiplayerLobby/Blueprints/GameModes/Base/Player/BP_PS_Base` _array_element))
        (if (`/Game/BeginnerMultiplayerLobby/Blueprints/GameModes/Base/Player/BP_PS_Base.IsReady` _asbp_ps_base)
          (set `self.ReadyCount` (+ (`self.ReadyCount`) 1))))))
  (set `self.StartCheck` (>= (`self.ReadyCount`) _numconnections)))

(fn `OnRep_AllPlayer`
  (bind _foundwidgets (`WidgetBlueprintLibrary.GetAllWidgetsOfClass` "/Game/BeginnerMultiplayerLobby/Widgets/Gameplay/PlayerList/WB_PlayerList.WB_PlayerList_C" false))
  (for _array_element _foundwidgets
    (`/Game/BeginnerMultiplayerLobby/Widgets/Gameplay/PlayerList/WB_PlayerList.Update_PlayerList` _array_element)))

(fn `OnRep_AllPlayers`
  ;[0.05448 0.05448 0.05448] Update all WB_PlayerList widgets
  (bind _foundwidgets (`WidgetBlueprintLibrary.GetAllWidgetsOfClass` "/Game/BeginnerMultiplayerLobby/Widgets/Gameplay/PlayerList/WB_PlayerList.WB_PlayerList_C" false))
  (for _array_element _foundwidgets
    (`/Game/BeginnerMultiplayerLobby/Widgets/Gameplay/PlayerList/WB_PlayerList.Update_PlayerList` _array_element)))

(fn `OnRep_CountDown`
  (`/Engine/EditorBlueprintResources/ActorMacros.Switch Has Authority`
    (:`Authority`
      ;[0.05098 0.05098 0.05098] Travel to the Gameplay Level when the countdown hit's zero. Otherwise continue the Countdown
      (if (`self.StartCheck`)
        (if (== (`self.CountDown`) 0)
          (bind _asbp_macs_pc (cast `/Game/MACS/Classes/BP_MACS_PC` (`GameplayStatics.GetPlayerController` 0)))
          (`/Game/MACS/Classes/BP_MACS_PC.SR_SpawnCharacter` _asbp_macs_pc)
          (else
            (`self.CountDownStart`)))))))

(fn `OnRep_StartCheck`
  (`/Engine/EditorBlueprintResources/ActorMacros.Switch Has Authority`
    (:`Authority`
      (if (`self.StartCheck`)
        (`self.CountDownStart`)))))

(fn `UserConstructionScript`)