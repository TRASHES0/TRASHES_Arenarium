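; Lobby game mode that moves all players from the lobby into the gameplay map through server travel.
; Its travel event notifies every player controller, then reads the map name from the session's extra settings.
; When a name is found, it creates a loading screen and waits briefly before traveling there.
; If the settings or name are missing, it travels straight to the default gameplay level without that screen or delay.
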(event `TravelTo_Gameplay_Level`
  ;[0.05098 0.05098 0.05098] Create a loading Screen on all players, then server travel to the Gameplay_Level
  (for _array_element (`self.All_PlayerControllers`)
    (`/Game/BeginnerMultiplayerLobby/Blueprints/GameModes/Base/Player/BP_PC_Base.ServerTravel` _array_element))
  (bind (_numconnections _numprivateconnections _bislan _bisdedicated _ballowinvites _ballowjoininprogress _bisanticheatenabled _builduniqueid _extrasettings) (`AdvancedSessionsLibrary.GetSessionSettings`)
    (:`OnSuccess`
      (bind _settingvalue (`AdvancedSessionsLibrary.GetSessionPropertyString` _extrasettings "MAPNAME")
        (:`Found`
          (`/Game/BeginnerMultiplayerLobby/Blueprints/FunctionLibrary/BP_FL_General.Create_LoadingScreen`)
          (`KismetSystemLibrary.Delay` 2.0) ; Loading screen vis time
          (`AdvancedSessionsLibrary.ServerTravel` _settingvalue true))
        (:`NotFound`
          (`AdvancedSessionsLibrary.ServerTravel` "Gameplay_Level" true :!label _label))))
    (:`OnFailure`
      (goto _label))))

(fn `UserConstructionScript`
  (`parent.UserConstructionScript`))