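; Lobby Game State that starts the match once all players are ready.
; Check_ReadyStatuses resets the countdown and counts ready lobby player states to set StartingGame, whose RepNotify starts the countdown on the server.
; Each one-second tick decrements StartCountDown, and its RepNotify re-triggers the tick, forming a loop without a timer that ends with BP_GM_Lobby travelling to the gameplay level at zero.
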(event `MatchStart_Countdown`
  ;[0.05098 0.05098 0.05098] Countdown the Match Start
  (`KismetSystemLibrary.Delay` 1.0)
  (set `self.StartCountDown` (- (`self.StartCountDown`) 1)))

(fn `Check_ReadyStatuses`
  (locals (AmountOfReadyPlayers :type Integer))
  ;[0.05098 0.05098 0.05098] Reset the Ready Status variables since we're checking again
  (set `self.AmountOfReady` 0)
  (set `self.StartCountDown` 10)
  (set `self.StartingGame?` false)
  ;[0.05098 0.05098 0.05098] Count the amount of players who's Ready Status is set to Ready. Then determine if we Start the Game Launch or not.
  (for _array_element (`self.AllPlayers`)
    (bind _asbp_ps_lobby (cast `/Game/BeginnerMultiplayerLobby/Blueprints/GameModes/Lobby/Player/BP_PS_Lobby` _array_element))
    (if (`/Game/BeginnerMultiplayerLobby/Blueprints/GameModes/Lobby/Player/BP_PS_Lobby.Ready?` _asbp_ps_lobby)
      (set `self.AmountOfReady` (+ (`self.AmountOfReady`) 1))))
  (set `self.StartingGame?` (>= (`self.AmountOfReady`) (`GameplayStatics.GetNumPlayerStates`))))

(fn `OnRep_StartCountDown`
  (`/Engine/EditorBlueprintResources/ActorMacros.Switch Has Authority`
    (:`Authority`
      (if (`self.StartingGame?`)
        ;[0.05098 0.05098 0.05098] Travel to the Gameplay Level when the countdown hit's zero. Otherwise continue the Countdown
        (if (== (`self.StartCountDown`) 0)
          (bind _asbp_gm_lobby (cast `/Game/BeginnerMultiplayerLobby/Blueprints/GameModes/Lobby/Core/BP_GM_Lobby` (`GameplayStatics.GetGameMode`)))
          (`/Game/BeginnerMultiplayerLobby/Blueprints/GameModes/Lobby/Core/BP_GM_Lobby.TravelTo_Gameplay_Level` _asbp_gm_lobby)
          (else
            (`self.MatchStart_Countdown`)))))))

(fn `OnRep_StartingGame?`
  ;[0.05098 0.05098 0.05098] If we are Starting the Game, then start the Match Countdown
  (`/Engine/EditorBlueprintResources/ActorMacros.Switch Has Authority`
    (:`Authority`
      (if (`self.StartingGame?`)
        (`self.MatchStart_Countdown`)))))

(fn `UserConstructionScript`
  (`parent.UserConstructionScript`))