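; BP_WIndArea is a wind zone actor that pushes any BP_Character_Base overlapping it.
; Begin overlap plays a timeline whose Wind track value is added to the character's location on every update, without sweep or delta-time scaling.
; End overlap by such a character stops that single shared timeline, and both events print debug strings.
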(event `self.ReceiveActorBeginOverlap`
  (params (OtherActor :type "Actor Object Reference"))
  (bind _asbp_character_base (cast `/Game/BeginnerMultiplayerLobby/Blueprints/Characters/BP_Character_Base` OtherActor))
  (`/Engine/EditorBlueprintResources/StandardMacros.IsValid` _asbp_character_base
    (:`Is Valid`
      (`KismetSystemLibrary.PrintString` "Begin Overlap")
      (bind (_direction _wind) (`Timeline|타임라인`)
        (:`Update`
          (`self.K2_SetActorLocation` _asbp_character_base (+ _wind (`self.K2_GetActorLocation` _asbp_character_base)) false false))))))

(event `self.ReceiveActorEndOverlap`
  (params (OtherActor :type "Actor Object Reference"))
  (bind _asbp_character_base (cast `/Game/BeginnerMultiplayerLobby/Blueprints/Characters/BP_Character_Base` OtherActor))
  (`/Engine/EditorBlueprintResources/StandardMacros.IsValid` _asbp_character_base
    (:`Is Valid`
      (`KismetSystemLibrary.PrintString` "End Overlap")
      (`TimelineComponent.Stop` (`self.타임라인`)))))

(fn `UserConstructionScript`)