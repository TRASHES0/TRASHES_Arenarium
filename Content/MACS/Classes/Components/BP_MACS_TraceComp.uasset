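; MACS actor component for melee hit detection, running sweep traces between StartTrace and StopTrace from anim notify states.
; On BeginPlay it turns the owner's mesh sockets named Trace_Box, Sphere, Capsule or Line into attached components, reading shape sizes from socket rotation and segmenting lines.
; A short delay loop traces each point from its last position.
; New hit actors trigger a GAS HitSomething event on the owning pawn, with a line-depth multiplier.
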(event `self.ReceiveBeginPlay`
  ;[1 1 1] SetRefs, Add Component by Mesh Ref and possibility of debug on editor if set true as default value;
  (`|ExecutionSequence`
    (:`then_0`
      (`self.SetRefs`))
    (:`then_1`
      (`self.AddStoreCompToTrace`))
    (:`then_2`
      ;;[1 1 1] This will keep enabled the traces debug. Disable this after setup the trace points
      (if (`self.DebugInEditor`)
        (`self.DebugTracesInEditor`)))))

(event `StartTrace`
  (params (TraceInfo :type "Array of /Game/MACS/DataModels/E_MACS_TraceInfo Structure"))
  ;[1 1 1] Make the trace loop while in the anim notify state
  (`KismetArrayLibrary.Array_Clear` (`self.HittedActors`))
  (`KismetArrayLibrary.Array_Clear` (`self.LastTracePositions`))
  (set `self.IsTracing` true)
  (`|ExecutionSequence`
    (:`then_0`
      (goto _label :!via `Open`))
    (:`then_1`
      (`/Engine/EditorBlueprintResources/StandardMacros.Gate` false :!label _label
        (:`Exit`
          (`|ExecutionSequence`
            (:`then_0`
              (if (or (`self.IsTracing`) (`self.DebugInEditor`))
                (`self.MakeTrace` TraceInfo)
                (else
                  (goto _label :!via `Close`))))
            (:`then_1`
              (`KismetSystemLibrary.Delay` 0.005)
              (goto _label))))))))

(event `StopTrace`
  ;[1 1 1] Finish the trace loop at end of anim notify state
  (set `self.IsTracing` false))

(fn `AddStoreCompToTrace`
  (locals (LocalMeshesRef :type "Array of /Game/MACS/DataModels/S_MACS_TracePoint Structure") (SocketNames :type "Array of Name"))
  (bind _returnvalue (`self.GetOwner`))
  (bind _tracepointsref (`self.TracePointsRef`))
  ;[1 1 1] Use the socket on each mesh ref to create a trace point
  (bind _output_get (set `local.LocalMeshesRef` _tracepointsref))
  (`KismetArrayLibrary.Array_Clear` _tracepointsref)
  (for _array_element _output_get
    (bind _meshcompref (break `/Game/MACS/DataModels/S_MACS_TracePoint` _array_element))
    (for _array_element_2 (`SceneComponent.GetAllSocketNames` _meshcompref)
      (bind _returnvalue_2 (`KismetStringLibrary.Conv_NameToString` _array_element_2))
      (bind _sceneclasstotrace (`self.GetSceneClassToTrace` _returnvalue_2))
      ;[1 1 1] Create the single or multiple trace points based on the type of each described on the socket name
      (if (`KismetSystemLibrary.IsValidClass` _sceneclasstotrace)
        (if (!= _sceneclasstotrace "/Script/Engine.SceneComponent")
          (bind _returnvalue_3 (`|AddComponentByClass` _returnvalue _sceneclasstotrace))
          (bind `_as씬_컴포넌트` (cast `SceneComponent` _returnvalue_3))
          (`KismetArrayLibrary.Array_AddUnique` (`self.TracePointsRef`) (make `/Game/MACS/DataModels/S_MACS_TracePoint` _meshcompref `_as씬_컴포넌트` _array_element_2))
          (else
            ;;[1 1 1] Create N mid line trace
            (for _index (range (+ (+ (`self.MidTracesPerSwing`) 1) 1))
              (bind _returnvalue_4 (`|AddComponentByClass` _returnvalue _sceneclasstotrace))
              (bind `_as씬_컴포넌트_2` (cast `SceneComponent` _returnvalue_4))
              (`KismetArrayLibrary.Array_AddUnique` (`self.TracePointsRef`) (make `/Game/MACS/DataModels/S_MACS_TracePoint` _meshcompref `_as씬_컴포넌트_2` (`KismetStringLibrary.Conv_StringToName` (`self.GetLinearTraceSocketNameByIndex` _index _returnvalue_2))))))))))
  (`self.ConfigTraceComp`))

(fn `CalculateDepthOnLinearTrace`
  (params (LinearSocketName :type Name))
  (returns (ReturnValue :type "Float (double-precision)"))
  (bind _returnvalue (+ (`self.MidTracesPerSwing`) 2))
  ;[1 1 1] Calculate Depth Trace. 1 when close to linear start socket and lower when away from this.
  (return (/ (* (/ 100 _returnvalue) (- _returnvalue (`self.GetLinearTraceIndex` (`KismetStringLibrary.Conv_NameToString` LinearSocketName)))) 100)))

(fn `ConfigActorComp`
  (params (MeshCompRef :type "MeshComponent Object Reference") (SceneCompRef :type "SceneComponent Object Reference") (SocketName :type Name))
  (`SceneComponent.K2_AttachToComponent` SceneCompRef MeshCompRef (select `bool` (`.bSuccess` (cast `SkeletalMeshComponent` MeshCompRef :!pure true)) :`true` SocketName) "KeepRelative" "KeepRelative" "KeepRelative" true)
  (`self.SetComponentTickEnabled` SceneCompRef false))

(fn `ConfigTraceComp`
  (for _array_element (`self.TracePointsRef`)
    (bind _returnvalue (`KismetStringLibrary.Conv_NameToString` (`.SocketName_21_A3A439734A14EF225A88448005F2C9D3` (break `/Game/MACS/DataModels/S_MACS_TracePoint` _array_element))))
    ;[1 1 1] If Linear Trace Point
    (if (not (`KismetStringLibrary.Contains` _returnvalue "Trace_Line"))
      ;[1 1 1] If Other Shape Comp
      (`self.SetRelativeTransformIfShape` (break `/Game/MACS/DataModels/S_MACS_TracePoint` _array_element) (`.SceneCompRef_34_0E5ED2B146470EF140CB36B0FA8E6464` (break `/Game/MACS/DataModels/S_MACS_TracePoint` _array_element)) (`.SocketName_21_A3A439734A14EF225A88448005F2C9D3` (break `/Game/MACS/DataModels/S_MACS_TracePoint` _array_element)))
      (`self.SetShapeSettings` (break `/Game/MACS/DataModels/S_MACS_TracePoint` _array_element) (`.SceneCompRef_34_0E5ED2B146470EF140CB36B0FA8E6464` (break `/Game/MACS/DataModels/S_MACS_TracePoint` _array_element)) (`.SocketName_21_A3A439734A14EF225A88448005F2C9D3` (break `/Game/MACS/DataModels/S_MACS_TracePoint` _array_element)))
      (else
        (`SceneComponent.K2_SetRelativeTransform` (`.SceneCompRef_34_0E5ED2B146470EF140CB36B0FA8E6464` (break `/Game/MACS/DataModels/S_MACS_TracePoint` _array_element)) (`self.GetTransformToSegmentTraceLine` (break `/Game/MACS/DataModels/S_MACS_TracePoint` _array_element) (`self.GetLinearTraceIndex` _returnvalue)) false false)))
    (`self.ConfigActorComp` (break `/Game/MACS/DataModels/S_MACS_TracePoint` _array_element) (`.SceneCompRef_34_0E5ED2B146470EF140CB36B0FA8E6464` (break `/Game/MACS/DataModels/S_MACS_TracePoint` _array_element)) (`.SocketName_21_A3A439734A14EF225A88448005F2C9D3` (break `/Game/MACS/DataModels/S_MACS_TracePoint` _array_element)))))

(fn `DebugTracesInEditor`
  (bind _debugtraceoneditor (`self.DebugTraceOnEditor`))
  (`|ExecutionSequence`
    (:`then_0`
      (`KismetArrayLibrary.Array_Clear` (`self.DebugTraceOnEditor`))
      (for _array_element (`self.TracePointsRef`)
        (`KismetArrayLibrary.Array_Add` _debugtraceoneditor (make `/Game/MACS/DataModels/E_MACS_TraceInfo` "NewEnumerator0" "NewEnumerator3" (`.SocketName_21_A3A439734A14EF225A88448005F2C9D3` (break `/Game/MACS/DataModels/S_MACS_TracePoint` _array_element)))))
      (`self.StartTrace` _debugtraceoneditor))
    (:`then_1`
      (`KismetSystemLibrary.K2_SetTimer` null "UpdateTraceCompTransform" 0.1 true))))

(fn `FilterTargetsAndSendGameplayEvent`
  (params (HitResults :type "Array of HitResult Structure") (LinearSocketName :type Name) (TraceInfo :type "/Game/MACS/DataModels/E_MACS_TraceInfo Structure"))
  (bind _linearsocketname (`local.LinearSocketName`))
  (bind _hittedactors (`self.HittedActors`))
  (bind (_traceinfo_controltype _traceinfo_damagetype) (break `/Game/MACS/DataModels/E_MACS_TraceInfo` (`local.TraceInfo`)))
  (bind _pawnref (`self.PawnRef`))
  (for _array_element HitResults
    (bind (_bblockinghit _binitialoverlap _time _distance _location _impactpoint _normal _impactnormal _physmat _hitactor _hitcomponent) (`GameplayStatics.BreakHitResult` _array_element))
    (bind _returnvalue (`GameplayStatics.GetObjectClass` _hitcomponent))
    (if (and (not (`KismetArrayLibrary.Array_IsValidIndex` _hittedactors (`KismetArrayLibrary.Array_Find` _hittedactors _hitactor))) (or (== _returnvalue "/Script/Engine.SkeletalMeshComponent") (== _returnvalue "/Script/Engine.StaticMeshComponent") (== _returnvalue "/Script/Engine.InstancedStaticMeshComponent")) (!= (`GameplayStatics.GetObjectClass` _hitactor) "/Game/MACS/Classes/BP_MACS_Inv_Item.BP_MACS_Inv_Item_C"))
      (`KismetArrayLibrary.Array_AddUnique` (`self.HittedActors`) _hitactor)
      ;[1 1 1] Sent gameplay event to Ability with data of target and dmg multiplier by trace
      (bind _returnvalue_2 (`|GenericCreateObject` _pawnref "/Game/MACS/Classes/BP_MACS_TraceInfo.BP_MACS_TraceInfo_C" (`|MakeArray` (make `/Game/MACS/DataModels/E_MACS_TraceInfo` _traceinfo_controltype _traceinfo_damagetype _linearsocketname (`self.CalculateDepthOnLinearTrace` _linearsocketname)) :!type "/Game/MACS/DataModels/E_MACS_TraceInfo Structure")))
      (`AbilitySystemBlueprintLibrary.SendGameplayEventToActor` (`self.PawnRef`) (struct :`TagName` "MACS_GAS.Abilities.Events.HitSomething") (make `GameplayEventData` (struct) _pawnref _hitactor _returnvalue_2 null (struct) (struct) (struct) 0.0 (`AbilitySystemBlueprintLibrary.AbilityTargetDataFromHitResult` _array_element)))
      (message `/Game/MACS/Classes/Interfaces/BPI_MACS_Projectile.HandleCollision` (`self.GetOwner`) _array_element))))

(fn `GetLinearTraceIndex`
  (params (SocketName :type String))
  (returns (LinearSocketIndex :type Integer))
  (return (`KismetStringLibrary.Conv_StringToInt` (`KismetStringLibrary.GetSubstring` SocketName (+ (`KismetStringLibrary.FindSubstring` SocketName "_" false true) 1) (`KismetStringLibrary.Len` (`KismetStringLibrary.Conv_IntToString` (+ (`self.MidTracesPerSwing`) 2)))))))

(fn `GetLinearTraceSocketNameByIndex`
  (params (LinearTraceIndex :type Integer) (StartSocketName :type String))
  (returns (LinearTraceSocketName :type String))
  (return (`KismetStringLibrary.Concat_StrStr` "Trace_Line_" (`KismetStringLibrary.Conv_IntToString` LinearTraceIndex))))

(fn `GetSceneClassToTrace`
  (params (SocketName :type String))
  (returns (SceneClassToTrace :type "ActorComponent Class Reference"))
  (locals (LocalCompToTraceClass :type "ActorComponent Class Reference"))
  (if (`KismetStringLibrary.Contains` SocketName "Trace_Box")
    (set `local.LocalCompToTraceClass` "/Script/Engine.BoxComponent")
    (elif (`KismetStringLibrary.Contains` SocketName "Trace_Sphere")
      (set `local.LocalCompToTraceClass` "/Script/Engine.SphereComponent")
      (elif (`KismetStringLibrary.Contains` SocketName "Trace_Capsule")
        (set `local.LocalCompToTraceClass` "/Script/Engine.CapsuleComponent")
        (elif (`KismetStringLibrary.Contains` SocketName "Trace_Line_Start")
          (set `local.LocalCompToTraceClass` "/Script/Engine.SceneComponent")
          (else
            (return null))))))
  (return (`local.LocalCompToTraceClass`)))

(fn `GetSocketNameByPartialName`
  (params (PrimitiveCompRef :type "PrimitiveComponent Object Reference") (PartialSocketName :type String))
  (returns (SocketNameFound :type Name))
  (for _array_element (`SceneComponent.GetAllSocketNames` PrimitiveCompRef)
    (if (`KismetStringLibrary.Contains` (`KismetStringLibrary.Conv_NameToString` _array_element) PartialSocketName)
      (return _array_element)))
  (return "None"))

(fn `GetTraceDmgBySocketName`
  (params (SocketName :type String))
  (returns (DmgType :type "/Game/MACS/DataModels/E_MACS_CollisionType Enum") (DmgPercentage :type Integer))
  (locals (LocalDmgType :type "/Game/MACS/DataModels/E_MACS_CollisionType Enum"))
  (if (`KismetStringLibrary.Contains` SocketName "_C_")
    (set `local.LocalDmgType` "NewEnumerator0")
    (elif (`KismetStringLibrary.Contains` SocketName "_S_")
      (set `local.LocalDmgType` "NewEnumerator1")
      (else
        (set `local.LocalDmgType` "NewEnumerator2"))))
  (return (`local.LocalDmgType`) (`KismetStringLibrary.Conv_StringToInt` (`KismetStringLibrary.GetSubstring` SocketName (+ (`KismetStringLibrary.FindSubstring` SocketName "_" false true) 1) 3))))

(fn `GetTransformToSegmentTraceLine`
  (params (MeshRef :type "MeshComponent Object Reference") (TraceIndex :type Integer))
  (returns (ReturnValue :type "Transform Structure"))
  (bind _returnvalue_location (`KismetMathLibrary.BreakTransform` (`SceneComponent.GetSocketTransform` MeshRef (`self.GetSocketNameByPartialName` MeshRef "Trace_Line_Start") "RTS_Component")))
  (return (`KismetMathLibrary.MakeTransform` (+ _returnvalue_location (* (`local.TraceIndex`) (`self.OffsetBetweenLinearTracesPoints` (`local.MeshRef`)))))))

(fn `InitialLocationsToTrace`
  (for _array_element (`self.TracePointsRef`)
    (`KismetArrayLibrary.Array_Add` (`self.LastTracePositions`) (`SceneComponent.K2_GetComponentLocation` (`.SceneCompRef_34_0E5ED2B146470EF140CB36B0FA8E6464` (break `/Game/MACS/DataModels/S_MACS_TracePoint` _array_element))))))

(fn `MakeTrace`
  (params (TraceInfo :type "Array of /Game/MACS/DataModels/E_MACS_TraceInfo Structure"))
  (locals (LastHit :type " Structure"))
  ;[1 1 1] Store the initial world location of each trace point and make a loop to trace each point desired/setted on the anim notify state
  (`self.InitialLocationsToTrace`)
  (for _array_element (`local.TraceInfo`)
    (for (_array_element_2 _array_index) (`self.TracePointsRef`)
      (if (and (`KismetStringLibrary.Contains` (`KismetStringLibrary.Conv_NameToString` (`.SocketName_21_A3A439734A14EF225A88448005F2C9D3` (break `/Game/MACS/DataModels/S_MACS_TracePoint` _array_element_2))) (`KismetStringLibrary.Conv_NameToString` (`.SocketsToTrace_22_9AF6591640F04366190CD98847C094A5` (break `/Game/MACS/DataModels/E_MACS_TraceInfo` _array_element)))) (not (`Actor.bHidden` (`self.GetOwner` (break `/Game/MACS/DataModels/S_MACS_TracePoint` _array_element_2)))))
        (bind `_as박스_콜리전` (cast `BoxComponent` (`.SceneCompRef_34_0E5ED2B146470EF140CB36B0FA8E6464` (break `/Game/MACS/DataModels/S_MACS_TracePoint` _array_element_2)))
          (:`then`
            (bind _outhits (`self.MultiBoxTrace` _array_index `_as박스_콜리전`))
            (`self.FilterTargetsAndSendGameplayEvent` _outhits "None" _array_element))
          (:`CastFailed`
            (bind `_as스피어_콜리전` (cast `SphereComponent` (`.SceneCompRef_34_0E5ED2B146470EF140CB36B0FA8E6464` (break `/Game/MACS/DataModels/S_MACS_TracePoint` _array_element_2)))
              (:`then`
                (bind _outhits_2 (`self.MultSphereTrace` _array_index `_as스피어_콜리전`))
                (`self.FilterTargetsAndSendGameplayEvent` _outhits_2 "None" _array_element))
              (:`CastFailed`
                (bind `_as캡슐_콜리전` (cast `CapsuleComponent` (`.SceneCompRef_34_0E5ED2B146470EF140CB36B0FA8E6464` (break `/Game/MACS/DataModels/S_MACS_TracePoint` _array_element_2)))
                  (:`then`
                    (bind _outhits_3 (`self.MultCapsuleTrace` _array_index `_as캡슐_콜리전`))
                    (`self.FilterTargetsAndSendGameplayEvent` _outhits_3 "None" _array_element))
                  (:`CastFailed`
                    (bind _outhits_4 (`self.MultiLineTrace` _array_index (`.SceneCompRef_34_0E5ED2B146470EF140CB36B0FA8E6464` (break `/Game/MACS/DataModels/S_MACS_TracePoint` _array_element_2))))
                    (`self.FilterTargetsAndSendGameplayEvent` _outhits_4 (`.SocketName_21_A3A439734A14EF225A88448005F2C9D3` (break `/Game/MACS/DataModels/S_MACS_TracePoint` _array_element_2)) _array_element)))))))))))

(fn `MultCapsuleTrace`
  (params (TraceIndex :type Integer) (CapsuleCompRef :type "CapsuleComponent Object Reference"))
  (returns (OutHits :type "Array of HitResult Structure"))
  (locals (LocaHitResults :type "Array of HitResult Structure"))
  (bind _returnvalue (`self.GetOwner`))
  (bind _capsulecompref (`local.CapsuleCompRef`))
  (bind _returnvalue_location (`KismetMathLibrary.BreakTransform` (`SceneComponent.K2_GetComponentToWorld` _capsulecompref)))
  (bind (_outradius _outhalfheight) (`CapsuleComponent.GetUnscaledCapsuleSize` _capsulecompref))
  ;[1 1 1] Multi Capsule Trace from the last world location to the current world location of the trace point
  (`|ExecutionSequence`
    (:`then_0`
      (bind _debugtrace (message `/Game/MACS/Classes/Interfaces/BPI_MACS_Character.GetDebugTrace` (`self.PawnRef`)))
      (bind _outhits (`KismetSystemLibrary.CapsuleTraceMultiForObjects` (`|GetArrayItem` (`self.LastTracePositions`) (`local.TraceIndex`)) _returnvalue_location (select `bool` (`.bSuccess` (cast `SkeletalMeshComponent` (`SceneComponent.GetAttachParent` _capsulecompref) :!pure true)) :`false` (/ _outradius 1.2) :`true` _outradius :!type "Float (double-precision)") _outhalfheight (`|MakeArray` "ObjectTypeQuery3" "ObjectTypeQuery1" "ObjectTypeQuery2" :!type "EObjectTypeQuery Enum") false (`|MakeArray` _returnvalue (`Actor.GetOwner` _returnvalue)) (select `bool` _debugtrace :`true` "ForDuration" :!type "EDrawDebugTrace Enum") true (struct :`R` 1.0 :`G` 1.0 :`A` 1.0) (struct :`G` 1.0 :`A` 1.0) (`self.DrawDebugTime`)))
      (set `local.LocaHitResults` _outhits))
    (:`then_1`
      (`KismetArrayLibrary.Array_Set` (`self.LastTracePositions`) (`local.TraceIndex`) (`SceneComponent.K2_GetComponentLocation` (`local.CapsuleCompRef`))))
    (:`then_2`
      (return (`local.LocaHitResults`)))))

(fn `MultiBoxTrace`
  (params (TraceIndex :type Integer) (BoxCompRef :type "BoxComponent Object Reference"))
  (returns (OutHits :type "Array of HitResult Structure"))
  (locals (LocalHitResults :type "Array of HitResult Structure"))
  (bind _returnvalue (`self.GetOwner`))
  (bind _boxcompref (`local.BoxCompRef`))
  (bind (_returnvalue_location _returnvalue_rotation) (`KismetMathLibrary.BreakTransform` (`SceneComponent.K2_GetComponentToWorld` _boxcompref)))
  (bind _boxextent (`BoxComponent.BoxExtent` _boxcompref))
  ;[1 1 1] Multi Box Trace from the last world location to the current world location of the trace point
  (`|ExecutionSequence`
    (:`then_0`
      (bind _debugtrace (message `/Game/MACS/Classes/Interfaces/BPI_MACS_Character.GetDebugTrace` (`self.PawnRef`)))
      (bind _outhits (`KismetSystemLibrary.BoxTraceMultiForObjects` (`|GetArrayItem` (`self.LastTracePositions`) (`local.TraceIndex`)) _returnvalue_location (select `bool` (`.bSuccess` (cast `SkeletalMeshComponent` (`SceneComponent.GetAttachParent` _boxcompref) :!pure true)) :`false` (/ _boxextent 1.3) :`true` _boxextent) _returnvalue_rotation (`|MakeArray` "ObjectTypeQuery3" "ObjectTypeQuery1" "ObjectTypeQuery2" :!type "EObjectTypeQuery Enum") false (`|MakeArray` _returnvalue (`Actor.GetOwner` _returnvalue)) (select `bool` _debugtrace :`true` "ForDuration" :!type "EDrawDebugTrace Enum") true (struct :`R` 1.0 :`B` 1.0 :`A` 1.0) (struct :`G` 1.0 :`A` 1.0) (`self.DrawDebugTime`)))
      (set `local.LocalHitResults` _outhits))
    (:`then_1`
      (`KismetArrayLibrary.Array_Set` (`self.LastTracePositions`) (`local.TraceIndex`) (`SceneComponent.K2_GetComponentLocation` (`local.BoxCompRef`))))
    (:`then_2`
      (return (`local.LocalHitResults`)))))

(fn `MultiLineTrace`
  (params (TraceIndex :type Integer) (SceneCompRef :type "SceneComponent Object Reference"))
  (returns (OutHits :type "Array of HitResult Structure"))
  (locals (LocaHitResults :type "Array of HitResult Structure"))
  (bind _returnvalue (`self.GetOwner`))
  (bind _returnvalue_location (`KismetMathLibrary.BreakTransform` (`SceneComponent.K2_GetComponentToWorld` (`local.SceneCompRef`))))
  ;[1 1 1] Multi Line Trace from the last world location to the current world location of the trace point
  (`|ExecutionSequence`
    (:`then_0`
      (bind _debugtrace (message `/Game/MACS/Classes/Interfaces/BPI_MACS_Character.GetDebugTrace` (`self.PawnRef`)))
      (bind _outhits (`KismetSystemLibrary.LineTraceMultiForObjects` (`|GetArrayItem` (`self.LastTracePositions`) (`local.TraceIndex`)) _returnvalue_location (`|MakeArray` "ObjectTypeQuery3" "ObjectTypeQuery1" "ObjectTypeQuery2" :!type "EObjectTypeQuery Enum") false (`|MakeArray` _returnvalue (`Actor.GetOwner` _returnvalue)) (select `bool` _debugtrace :`true` "ForDuration" :!type "EDrawDebugTrace Enum") true (struct :`R` 1.0 :`A` 1.0) (struct :`G` 1.0 :`A` 1.0) (`self.DrawDebugTime`)))
      (set `local.LocaHitResults` _outhits))
    (:`then_1`
      (`KismetArrayLibrary.Array_Set` (`self.LastTracePositions`) (`local.TraceIndex`) (`SceneComponent.K2_GetComponentLocation` (`local.SceneCompRef`))))
    (:`then_2`
      (return (`local.LocaHitResults`)))))

(fn `MultSphereTrace`
  (params (TraceIndex :type Integer) (SphereCompRef :type "SphereComponent Object Reference"))
  (returns (OutHits :type "Array of HitResult Structure"))
  (locals (LocalHitResults :type "Array of HitResult Structure"))
  (bind _spherecompref (`local.SphereCompRef`))
  (bind _returnvalue_location (`KismetMathLibrary.BreakTransform` (`SceneComponent.K2_GetComponentToWorld` _spherecompref)))
  (bind _sphereradius (`SphereComponent.SphereRadius` _spherecompref))
  ;[1 1 1] Multi Sphere Trace from the last world location to the current world location of the trace point
  (`|ExecutionSequence`
    (:`then_0`
      (bind _debugtrace (message `/Game/MACS/Classes/Interfaces/BPI_MACS_Character.GetDebugTrace` (`self.PawnRef`)))
      (bind _outhits (`KismetSystemLibrary.SphereTraceMultiForObjects` (`|GetArrayItem` (`self.LastTracePositions`) (`local.TraceIndex`)) _returnvalue_location (select `bool` (`.bSuccess` (cast `SkeletalMeshComponent` (`SceneComponent.GetAttachParent` _spherecompref) :!pure true)) :`false` (/ _sphereradius 1.6) :`true` _sphereradius :!type "Float (single-precision)") (`|MakeArray` "ObjectTypeQuery3" "ObjectTypeQuery1" "ObjectTypeQuery2" :!type "EObjectTypeQuery Enum") false (`|MakeArray` (`self.GetOwner`) (`self.PawnRef`)) (select `bool` _debugtrace :`true` "ForDuration" :!type "EDrawDebugTrace Enum") true (struct :`G` 1.0 :`B` 1.0 :`A` 1.0) (struct :`G` 1.0 :`A` 1.0) (`self.DrawDebugTime`)))
      (set `local.LocalHitResults` _outhits))
    (:`then_1`
      (`KismetArrayLibrary.Array_Set` (`self.LastTracePositions`) (`local.TraceIndex`) (`SceneComponent.K2_GetComponentLocation` (`local.SphereCompRef`))))
    (:`then_2`
      (return (`local.LocalHitResults`)))))

(fn `OffsetBetweenLinearTracesPoints`
  (params (PrimitiveCompRef :type "PrimitiveComponent Object Reference"))
  (returns (DistancesBetweenTraces :type "Vector Structure"))
  (bind _primitivecompref (`local.PrimitiveCompRef`))
  (bind _returnvalue_location (`KismetMathLibrary.BreakTransform` (`SceneComponent.GetSocketTransform` _primitivecompref (`self.GetSocketNameByPartialName` PrimitiveCompRef "Trace_Line_End") "RTS_Component")))
  (bind _returnvalue_location_2 (`KismetMathLibrary.BreakTransform` (`SceneComponent.GetSocketTransform` _primitivecompref (`self.GetSocketNameByPartialName` PrimitiveCompRef "Trace_Line_Start") "RTS_Component")))
  ;[1 1 1] Example: StartTrace(y) = 0; EndTrace(x) = 100; MidTracesPerSwing == 3. Formula: ( x - y )  / MidTracePerSwing + 1 = offset
  (return (/ (- _returnvalue_location _returnvalue_location_2) (+ (`self.MidTracesPerSwing`) 1))))

(fn `SetRefs`
  (bind _returnvalue (`self.GetOwner`))
  (bind _returnvalue_2 (`Actor.GetOwner` _returnvalue))
  (`|ExecutionSequence`
    (:`then_0`
      ;[1 1 1] Set Pawn Ref
      (set `self.PawnRef` (select `bool` (`KismetMathLibrary.ClassIsChildOf` (`GameplayStatics.GetObjectClass` _returnvalue) "/Script/Engine.Pawn") :`false` (select `bool` (`KismetMathLibrary.ClassIsChildOf` (`GameplayStatics.GetObjectClass` _returnvalue_2) "/Script/Engine.Pawn") :`false` (`Actor.Instigator` _returnvalue) :`true` _returnvalue_2 :!type "Actor Object Reference") :`true` _returnvalue)))
    (:`then_1`
      ;[1 1 1] Set Meshes Ref
      (for _array_element (`Actor.K2_GetComponentsByClass` (`self.GetOwner`) "/Script/Engine.MeshComponent")
        (if (not (`SceneComponent.bHiddenInGame` _array_element))
          (`KismetArrayLibrary.Array_AddUnique` (`self.TracePointsRef`) (make `/Game/MACS/DataModels/S_MACS_TracePoint` _array_element null)))))))

(fn `SetRelativeTransformIfShape`
  (params (MeshCompRef :type "MeshComponent Object Reference") (SceneCompRef :type "SceneComponent Object Reference") (SocketName :type Name))
  (bind _returnvalue_location (`KismetMathLibrary.BreakTransform` (`SceneComponent.GetSocketTransform` MeshCompRef SocketName "RTS_Component")))
  (`SceneComponent.K2_SetRelativeTransform` (`local.SceneCompRef`) (select `bool` (`.bSuccess` (cast `SkeletalMeshComponent` (`local.MeshCompRef`) :!pure true)) :`false` (`KismetMathLibrary.MakeTransform` _returnvalue_location) :!type "Transform Structure") false false)
  (return))

(fn `SetShapeSettings`
  (params (MeshCompRef :type "MeshComponent Object Reference") (SceneCompRef :type "SceneComponent Object Reference") (SocketName :type Name))
  (bind _meshcompref (`local.MeshCompRef`))
  (bind (_returnvalue_location _returnvalue_rotation) (`KismetMathLibrary.BreakTransform` (`SceneComponent.GetSocketTransform` _meshcompref SocketName "RTS_Component")))
  (bind (_returnvalue_location_2 _returnvalue_rotation_2) (`KismetMathLibrary.BreakTransform` (`SceneComponent.GetSocketTransform` _meshcompref SocketName "RTS_ParentBoneSpace")))
  (bind _roll (.roll (select `bool` (`.bSuccess` (cast `SkeletalMeshComponent` (`local.MeshCompRef`) :!pure true)) :`false` _returnvalue_rotation :`true` _returnvalue_rotation_2)))
  (bind _pitch (.pitch (select `bool` (`.bSuccess` (cast `SkeletalMeshComponent` (`local.MeshCompRef`) :!pure true)) :`false` _returnvalue_rotation :`true` _returnvalue_rotation_2)))
  (bind `_as박스_콜리전` (cast `BoxComponent` SceneCompRef)
    (:`then`
      ;[1 1 1] Set Shape parameter by the socket rotation
      (`BoxComponent.SetBoxExtent` `_as박스_콜리전` (`KismetMathLibrary.MakeVector` _roll _pitch (.yaw (select `bool` (`.bSuccess` (cast `SkeletalMeshComponent` (`local.MeshCompRef`) :!pure true)) :`false` _returnvalue_rotation :`true` _returnvalue_rotation_2))) true))
    (:`CastFailed`
      (bind `_as스피어_콜리전` (cast `SphereComponent` SceneCompRef)
        (:`then`
          (`SphereComponent.SetSphereRadius` `_as스피어_콜리전` _roll true))
        (:`CastFailed`
          (bind `_as캡슐_콜리전` (cast `CapsuleComponent` SceneCompRef))
          (`CapsuleComponent.SetCapsuleSize` `_as캡슐_콜리전` _roll _pitch true))))))

(fn `UpdateTraceCompTransform`
  (`self.ConfigTraceComp`))