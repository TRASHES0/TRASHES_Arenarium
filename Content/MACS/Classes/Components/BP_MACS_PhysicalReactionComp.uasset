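; Actor component that gives its owner's skeletal mesh a temporary physics-driven reaction to hits.
; BeginPlay adds a PhysicalAnimationComponent and binds it to that mesh.
; PhysicalHitReaction extends a timer, simulates bodies below the pelvis and applies a trace-direction impulse at the hit bone, redirecting pelvis hits to spine_01.
; Tick decays the timer into the physics blend weight, then stops simulation and disables itself.
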(event `self.ReceiveBeginPlay`
  (bind _returnvalue (`self.GetOwner`))
  ;[1 1 1] Set Refs
  (bind _returnvalue_2 (`|AddComponentByClass` _returnvalue "/Script/Engine.PhysicalAnimationComponent"))
  (bind _output_get (set `self.PhysicalCompRef` _returnvalue_2))
  (bind _output_get_2 (set `self.SkeletalMeshRef` (`Actor.GetComponentByClass` _returnvalue "/Script/Engine.SkeletalMeshComponent")))
  (`PhysicalAnimationComponent.SetSkeletalMeshComponent` _output_get _output_get_2))

(event `self.ReceiveTick`
  (params (DeltaSeconds :type "Float (single-precision)"))
  (bind _returnvalue (* DeltaSeconds 3.0))
  ;[1 1 1] Tick Physical Reaction
  (bind _output_get (set `self.HitReactionTimeRemaning` (- (`KismetMathLibrary.FInterpTo` (`self.HitReactionTimeRemaning`) 0.0 _returnvalue 1.0) _returnvalue)))
  (if (<= _output_get 0.0)
    (set `self.HitReactionTimeRemaning` 0.0)
    (`SkeletalMeshComponent.SetAllBodiesBelowSimulatePhysics` (`self.SkeletalMeshRef`) "pelvis" false true)
    (`self.SetComponentTickEnabled` false)
    (else
      (`SkeletalMeshComponent.SetAllBodiesBelowPhysicsBlendWeight` (`self.SkeletalMeshRef`) "pelvis" (`KismetMathLibrary.FMin` (`self.HitReactionTimeRemaning`) 1.0) false true))))

(event `PhysicalHitReaction`
  (params (HitResult :type "HitResult Structure (by ref)"))
  (bind (_bblockinghit _binitialoverlap _time _distance _location _impactpoint _normal _impactnormal _physmat _hitactor _hitcomponent _hitbonename _bonename _hititem _elementindex _faceindex _tracestart _traceend) (`GameplayStatics.BreakHitResult` HitResult))
  ;[1 1 1] Setup Physical Component
  (`self.SetComponentTickEnabled` true)
  (set `self.HitReactionTimeRemaning` (+ (`self.HitReactionTimeRemaning`) 2.0))
  ;[1 1 1] Add impulse to bone hitted
  (`SkeletalMeshComponent.SetAllBodiesBelowSimulatePhysics` (`self.SkeletalMeshRef`) "pelvis" true false)
  (`PrimitiveComponent.AddImpulse` (`self.SkeletalMeshRef`) (* (`KismetMathLibrary.Normal` (- _traceend _tracestart)) 5000) (select `bool` (== _hitbonename "pelvis") :`false` _hitbonename :`true` "spine_01") false))