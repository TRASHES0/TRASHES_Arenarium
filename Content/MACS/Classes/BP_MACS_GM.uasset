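; Game mode for the MACS demo, providing player respawn plus test utilities for AI, weapon items and game speed.
; It spawns behavior-tree AI at spawn refs of other teams, or in front of the pawn if none exist, each with a random weapon item nearby.
; Helpers remove AI and unequipped items, toggle an AI flag, and cycle global time dilation through nested FlipFlops.
; Restarting players are respawned through the MACS player controller.
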(event `self.ReceiveBeginPlay`
  (`KismetSystemLibrary.Delay` 0.2)
  (for _array_element (`GameStateBase.PlayerArray` (`GameplayStatics.GetGameState`))
    (`KismetSystemLibrary.PrintString` (`KismetStringLibrary.Conv_IntToString` (`PlayerState.PlayerId` _array_element)))))

(event `SetGlobalTimerDilation`
  (`/Engine/EditorBlueprintResources/StandardMacros.FlipFlop` :!label _label
    (:`A`
      (`/Engine/EditorBlueprintResources/StandardMacros.FlipFlop`
        (:`A`
          (`self.SetTimeDilation` 0.5))
        (:`B`
          (goto _label))))
    (:`B`
      (`/Engine/EditorBlueprintResources/StandardMacros.FlipFlop`
        (:`A`
          (`self.SetTimeDilation` 0.1))
        (:`B`
          (`self.SetTimeDilation` 1.0))))))

(event `self.K2_OnRestartPlayer`
  (params (NewPlayer :type "Controller Object Reference"))
  (bind _asbp_macs_pc (cast `/Game/MACS/Classes/BP_MACS_PC` NewPlayer))
  (`/Game/MACS/Classes/BP_MACS_PC.RespawnOnServer` _asbp_macs_pc))

(fn `RemoveAllAI`
  ;[1 1 1] Destroy AI pawn, controller and AI Player State if is valid
  (bind _outactors (`GameplayStatics.GetAllActorsOfClass` "/Script/Engine.Character"))
  (for _array_element _outactors
    (if (not (`Pawn.IsPlayerControlled` _array_element))
      (`self.K2_DestroyActor` (`AIBlueprintHelperLibrary.GetAIController` _array_element))
      (bind _playerstate (`Pawn.PlayerState` _array_element)
        (:`then`
          (`self.K2_DestroyActor` _playerstate))
        (:`else`
          _))
      (`self.K2_DestroyActor` _array_element)))
  (`KismetSystemLibrary.PrintString` "All AI Removed" true true (struct :`G` 1.0 :`A` 1.0)))

(fn `RemoveAllWeaponClasses`
  (bind _outactors (`GameplayStatics.GetAllActorsOfClass` "/Game/MACS/Classes/BP_MACS_Inv_Item.BP_MACS_Inv_Item_C"))
  (for _array_element _outactors
    (if (not (`/Game/MACS/Classes/BP_MACS_Inv_Item.EquippedItem` _array_element))
      (`self.K2_DestroyActor` _array_element))))

(fn `SetTimeDilation`
  (params (TimeDilation :type "Float (single-precision)"))
  (`GameplayStatics.SetGlobalTimeDilation` TimeDilation)
  (`KismetSystemLibrary.PrintString` (`KismetStringLibrary.Concat_StrStr` "Global Time Dilation: " (`KismetStringLibrary.Conv_DoubleToString` TimeDilation))))

(fn `SpawnAiWeaponClassByTeamID`
  (params (PawnRef :type "Actor Object Reference"))
  (bind _pawnref (`local.PawnRef`))
  (bind (_returnvalue_location _returnvalue_rotation) (`KismetMathLibrary.BreakTransform` (`self.GetTransform` _pawnref)))
  (bind _outactors (`GameplayStatics.GetAllActorsOfClass` "/Game/MACS/Classes/BP_MACS_SpawnRef.BP_MACS_SpawnRef_C"))
  ;[1 1 1] Spawn at front of player character if don't exist any spawn point like as in the MACS Demo Level
  (if (`KismetArrayLibrary.Array_IsEmpty` _outactors)
    (bind _returnvalue (`AIBlueprintHelperLibrary.SpawnAIFromClass` (`self.DefaultPawnClass`) "/Game/MACS/AI/BT_MACS_Demo.BT_MACS_Demo" (+ _returnvalue_location (* (`self.GetActorForwardVector` _pawnref) 100)) _returnvalue_rotation false self))
    (`/Engine/EditorBlueprintResources/StandardMacros.IsValid` _returnvalue
      (:`Is Valid`
        (message `/Game/MACS/Classes/Interfaces/BPI_MACS_Character.SetTeamID` _returnvalue -1)
        (`self.SpawnWeaponClass` _returnvalue (`KismetArrayLibrary.Array_Random` (`|MakeArray` 1 3 4 2 5)))))
    (else
      ;[1 1 1] Spawn AIs, set the TeamID and spawn the AI Controller to posses
      (for _array_element _outactors
        (bind _teamid (message `/Game/MACS/Classes/Interfaces/BPI_MACS_Character.GetTeamID` (`local.PawnRef`)))
        (if (!= (`/Game/MACS/Classes/BP_MACS_SpawnRef.TeamIdRef` _array_element) _teamid)
          (bind (_returnvalue_location_2 _returnvalue_rotation_2) (`KismetMathLibrary.BreakTransform` (`self.GetTransform` _array_element)))
          (bind _returnvalue_2 (`AIBlueprintHelperLibrary.SpawnAIFromClass` (`self.DefaultPawnClass`) "/Game/MACS/AI/BT_MACS_Demo.BT_MACS_Demo" _returnvalue_location_2 _returnvalue_rotation_2 false self))
          (`/Engine/EditorBlueprintResources/StandardMacros.IsValid` _returnvalue_2
            (:`Is Valid`
              (message `/Game/MACS/Classes/Interfaces/BPI_MACS_Character.SetTeamID` _returnvalue_2 (`/Game/MACS/Classes/BP_MACS_SpawnRef.TeamIdRef` _array_element))
              (`self.SpawnWeaponClass` _array_element (`KismetArrayLibrary.Array_Random` (`|MakeArray` 1 3 4 2 5))))))))))

(fn `SpawnWeaponClass`
  (params (SpawnActorRef :type "Actor Object Reference") (ItemID :type Integer))
  ;[1 1 1] Spawn WeaponClass
  (`|SpawnActorFromClass` "/Game/MACS/Classes/BP_MACS_Inv_Item.BP_MACS_Inv_Item_C" (`KismetMathLibrary.MakeTransform` (+ (`self.K2_GetActorLocation` SpawnActorRef) (* (`self.GetActorForwardVector` SpawnActorRef) 150))) "AdjustIfPossibleButAlwaysSpawn" "OverrideRootScale" null ItemID 1 false null))

(fn `ToggleEnableAI`
  (bind _output_get (set `self.EnableAI` (not (`self.EnableAI`))))
  (`KismetSystemLibrary.PrintString` (`KismetStringLibrary.Concat_StrStr` "EnableAI setted as " (`KismetStringLibrary.Conv_BoolToString` _output_get)) true true (struct :`G` 1.0 :`A` 1.0)))

(fn `UserConstructionScript`)